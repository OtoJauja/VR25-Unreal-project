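; AI controller for guards that runs BT_GuardBehavior and feeds it what the guard sees and hears.
; Perception updates route by sense class name into HandleSense, which writes the investigating flag and target keys to the Blackboard.
; Seeing the player sets them as target actor and raises walk speed, with no reset here.
; Losing sight clears that actor and stores the last stimulus location; hearing stores the noise location.
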(event `self.ReceiveBeginPlay`
  ; Begin Behaviour tree
  (`self.RunBehaviorTree` "/Game/AI/BT_GuardBehavior.BT_GuardBehavior"))

(event `self.AIPerception.OnTargetPerceptionUpdated`
  (params (Actor :type "Actor Object Reference") (Stimulus :type "AIStimulus Structure"))
  ; If AI perception activated then Does function Handle Sense
  (bind _returnvalue (`AIPerceptionSystem.GetSenseClassForStimulus` Stimulus))
  (`self.HandleSense` (`KismetSystemLibrary.GetClassDisplayName` _returnvalue) Stimulus Actor))

(fn `HandleSense`
  (params (Selection :type String) (Stimulus :type "AIStimulus Structure") (SensedActor :type "Actor Object Reference"))
  (bind (_stimulus_age _stimulus_expirationage _stimulus_strength _stimulus_stimuluslocation _stimulus_receiverlocation _stimulus_tag _stimulus_bsuccessfullysensed) (break `AIStimulus` (`local.Stimulus`)))
  (bind (_stimulus_age_2 _stimulus_expirationage_2 _stimulus_strength_2 _stimulus_stimuluslocation_2 _stimulus_receiverlocation_2 _stimulus_tag_2 _stimulus_bsuccessfullysensed_2) (break `AIStimulus` (`local.Stimulus`)))
  (bind (_stimulus_age_3 _stimulus_expirationage_3 _stimulus_strength_3 _stimulus_stimuluslocation_3) (break `AIStimulus` (`local.Stimulus`)))
  (bind (_stimulus_age_4 _stimulus_expirationage_4 _stimulus_strength_4 _stimulus_stimuluslocation_4) (break `AIStimulus` (`local.Stimulus`)))
  ; Checks for which sense is activated
  (switch `string` Selection
    (:`AiSense_Sight`
      (`BlackboardComponent.SetValueAsBool` (`self.Blackboard`) "IsInvestigating" _stimulus_bsuccessfullysensed_2)
      (if _stimulus_bsuccessfullysensed_2
        ; If seen then the Guard chases the player by finding location and the Guards Walk Speed is increased
        (if (== (`local.SensedActor`) (`GameplayStatics.GetPlayerCharacter` 0))
          (`BlackboardComponent.SetValueAsObject` (`self.Blackboard`) "TargetLocationActor" (`local.SensedActor`))
          (bind _ascharacter (cast `Character` (`self.K2_GetPawn`)))
          (set `CharacterMovementComponent.MaxWalkSpeed` 400.0 (`Character.CharacterMovement` _ascharacter)))
        (else
          ; If not then go back to normal AI wandering
          (`BlackboardComponent.SetValueAsVector` (`self.Blackboard`) "TargetLocationVector" _stimulus_stimuluslocation_3)
          (`BlackboardComponent.SetValueAsObject` (`self.Blackboard`) "TargetLocationActor" null))))
    (:`AiSense_Hearing`
      ; Moves to location where Player last made sound and is not seen
      (`BlackboardComponent.SetValueAsBool` (`self.Blackboard`) "IsInvestigating" _stimulus_bsuccessfullysensed)
      (`BlackboardComponent.SetValueAsVector` (`self.Blackboard`) "TargetLocationVector" _stimulus_stimuluslocation_4))))

(fn `UserConstructionScript`)