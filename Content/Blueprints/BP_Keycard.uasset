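; BP_Keycard is an interactable keycard pickup that unlocks a linked door for the player.
; On Interact it calls PickUpKeyMessage on its Door reference, prints a debug inventory message, plays a pickup sound and destroys itself.
; GetInteractionPromt supplies the "steal keycard" prompt text; no inventory is actually updated here.
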(event `/Game/Blueprints/BPI_Interact.Interact`
  (params (Interactor :type "Actor Object Reference"))
  ; Interact with Object, Activate Door bool to true
  (message `/Game/Blueprints/BPI_Door.Pick Up Key` (`self.Door`))
  (`KismetSystemLibrary.PrintString` (`KismetTextLibrary.Conv_TextToString` (`|FormatText` "Added {itemName} to the inventory of {actorName} " (`KismetSystemLibrary.GetDisplayName` self) (`KismetSystemLibrary.GetDisplayName` Interactor))))
  (`GameplayStatics.PlaySoundAtLocation` "/Game/Sounds/key_pickup.key_pickup" (`self.K2_GetActorLocation`) (struct) 1.0 1.0 0.0 null null null null)
  (`self.K2_DestroyActor`))

(fn `GetInteractionPromt`
  (returns (Value :type Text))
  (return "steal keycard"))

(fn `UserConstructionScript`)