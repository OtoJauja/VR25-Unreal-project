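; BP_VaultDoor is an interactable vault door that opens only after its key card has been picked up.
; PickUpKey sets HasKeyCard, which Interact checks before calling OpenDoor, playing a sci-fi opening sound and setting a short lifespan that destroys the actor.
; OpenDoor uses a timeline to lerp the Door component upward along relative Z.
; GetInteractionPromt supplies the "open Vault" prompt text.
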(event `OpenDoor`
  ; Door Animation
  (bind (_direction _door_float) (`Timeline|Open Door Timeline`)
    (:`Update`
      (`SceneComponent.K2_SetRelativeLocation` (`self.Door`) (`KismetMathLibrary.MakeVector` 0.0 0.0 (`KismetMathLibrary.Lerp` 0.0 360.0 _door_float)) false false))))

(event `/Game/Blueprints/BPI_Interact.Interact`
  (params (Interactor :type "Actor Object Reference"))
  ; Interact with door to open and check if door has key card is true
  (if (`self.HasKeyCard`)
    (`self.OpenDoor`)
    (`GameplayStatics.PlaySoundAtLocation` "/Game/Sounds/scifi-door-opening.scifi-door-opening" (`self.K2_GetActorLocation`) (struct) 1.0 1.0 0.0 null null null null)
    (`self.SetLifeSpan` 0.8)))

(event `/Game/Blueprints/BPI_Door.Pick Up Key`
  ; Interact with door to open and check if door has key card is true
  (set `self.HasKeyCard` true))

(fn `GetInteractionPromt`
  (returns (Value :type Text))
  (return "open Vault"))

(fn `UserConstructionScript`)